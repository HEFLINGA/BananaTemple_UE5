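; Treasure chest that opens when the player character walks into its collision box and ejects a health pickup.
; BeginPlay caches the ThirdPersonCharacter, and the box overlap compares against it before passing a DoOnce, so the chest opens only once.
; A timeline rotates the lid around its roll axis, then SpawnItems spawns the pickup at SpawnPoint, enables physics and launches it mostly upward with an impulse.
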(event `self.ReceiveBeginPlay`
  ;[1 1 1] Create Player Reference
  (bind _asbp_third_person_character (cast `/Game/MyProject/Blueprints/BP_ThirdPersonCharacter` (`GameplayStatics.GetPlayerCharacter` 0)))
  (set `self.Player Reference` _asbp_third_person_character))

(event `self.Box_Collision.OnComponentBeginOverlap`
  (params (OverlappedComponent :type "PrimitiveComponent Object Reference") (OtherActor :type "Actor Object Reference") (OtherComp :type "PrimitiveComponent Object Reference") (OtherBodyIndex :type Integer) (bFromSweep :type Boolean) (SweepResult :type "HitResult Structure (by ref)"))
  (bind _lid (`self.Lid`))
  (bind (_relativerotation_roll _relativerotation_pitch _relativerotation_yaw) (`KismetMathLibrary.BreakRotator` (`SceneComponent.RelativeRotation` _lid)))
  ;[1 1 1] Lid Open
  (if (== OtherActor (`self.Player Reference`))
    (`/Engine/EditorBlueprintResources/StandardMacros.DoOnce` false
      (:`Completed`
        (bind (_direction _xrotation) (`Timeline|OpenLid_TimeLine`)
          (:`Update`
            (`SceneComponent.K2_SetRelativeRotation` _lid (`KismetMathLibrary.MakeRotator` (* _xrotation -1.0) _relativerotation_pitch _relativerotation_yaw) false false))
          (:`Finished`
            (`self.SpawnItems`)))))))

(event `SpawnItems`
  (bind _returnvalue (`|SpawnActorFromClass` "/Game/MyProject/Blueprints/BP_HealthPickup.BP_HealthPickup_C" (`SceneComponent.K2_GetComponentToWorld` (`self.SpawnPoint`)) "Undefined" "OverrideRootScale" null null))
  (bind _sm_healthpickup (`/Game/MyProject/Blueprints/BP_HealthPickup.SM_HealthPickup` _returnvalue))
  (`PrimitiveComponent.SetSimulatePhysics` _sm_healthpickup true)
  (`PrimitiveComponent.AddImpulseAtLocation` _sm_healthpickup (500.0 0.0 6000.0) (`self.K2_GetActorLocation` _returnvalue) "None"))

(fn `UserConstructionScript`)