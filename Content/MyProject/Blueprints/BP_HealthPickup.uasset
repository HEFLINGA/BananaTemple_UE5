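; BP_HealthPickup is a pickup actor that restores health to the player character when touched.
; On BeginPlay it caches the player as a BP_ThirdPersonCharacter reference.
; When that player begins overlapping the SC_Collision component, it adds HealAmount to CurrentHealth, clamped between fixed limits, then destroys itself.
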(event `self.ReceiveBeginPlay`
  ;[1 1 1] Create Player Reference
  (bind _asbp_third_person_character (cast `/Game/MyProject/Blueprints/BP_ThirdPersonCharacter` (`GameplayStatics.GetPlayerCharacter` 0)))
  (set `self.Player Reference` _asbp_third_person_character))

(event `self.SC_Collision.OnComponentBeginOverlap`
  (params (OverlappedComponent :type "PrimitiveComponent Object Reference") (OtherActor :type "Actor Object Reference") (OtherComp :type "PrimitiveComponent Object Reference") (OtherBodyIndex :type Integer) (bFromSweep :type Boolean) (SweepResult :type "HitResult Structure (by ref)"))
  ;[1 1 1] Heal Player On Health Pickup
  (if (== OtherActor (`self.Player Reference`))
    (set `/Game/MyProject/Blueprints/BP_ThirdPersonCharacter.CurrentHealth` (`KismetMathLibrary.FClamp` (+ (`/Game/MyProject/Blueprints/BP_ThirdPersonCharacter.CurrentHealth` (`self.Player Reference`)) (`self.HealAmount`)) 0.0 100.0) (`self.Player Reference`))
    (`self.K2_DestroyActor`)))

(fn `UserConstructionScript`)