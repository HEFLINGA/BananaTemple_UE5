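; BP_Button is a floor-style button actor that moves down while the player character overlaps its sphere trigger.
; On BeginPlay it caches the player as a BP_ThirdPersonCharacter reference, so overlaps from other actors are ignored.
; Entering the sphere plays ButtonDown_Timeline, whose ZHeight track drives the button mesh's relative Z, and leaving reverses it.
; The file shows only this movement, with no action triggered by the press.
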(event `self.ReceiveBeginPlay`
  ;[1 1 1] Create Player Reference
  (bind _asbp_third_person_character (cast `/Game/MyProject/Blueprints/BP_ThirdPersonCharacter` (`GameplayStatics.GetPlayerCharacter` 0)))
  (set `self.Player Reference` _asbp_third_person_character))

(event `self.Sphere.OnComponentBeginOverlap`
  (params (OverlappedComponent :type "PrimitiveComponent Object Reference") (OtherActor :type "Actor Object Reference") (OtherComp :type "PrimitiveComponent Object Reference") (OtherBodyIndex :type Integer) (bFromSweep :type Boolean) (SweepResult :type "HitResult Structure (by ref)"))
  (bind _sm_button (`self.SM_Button`))
  (bind (_relativelocation_x _relativelocation_y) (`KismetMathLibrary.BreakVector` (`SceneComponent.RelativeLocation` _sm_button)))
  (if (== OtherActor (`self.Player Reference`))
    (bind (_direction _zheight) (`Timeline|ButtonDown_Timeline` :!label _label)
      (:`Update`
        (`SceneComponent.K2_SetRelativeLocation` _sm_button (`KismetMathLibrary.MakeVector` _relativelocation_x _relativelocation_y _zheight) false false)))))

(event `self.Sphere.OnComponentEndOverlap`
  (params (OverlappedComponent :type "PrimitiveComponent Object Reference") (OtherActor :type "Actor Object Reference") (OtherComp :type "PrimitiveComponent Object Reference") (OtherBodyIndex :type Integer))
  (if (== OtherActor (`self.Player Reference`))
    (goto _label :!via `Reverse`)))

(fn `UserConstructionScript`)