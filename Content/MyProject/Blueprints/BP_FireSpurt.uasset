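; BP_FireSpurt is a fire outlet that shows a spurt of fire when the player is near it.
; BeginPlay caches the player's BP_ThirdPersonCharacter so overlaps on BC_FireOutlet respond only to that character.
; Entering the volume reveals FireOut after a brief delay, and leaving hides it after a longer one.
; The graph only toggles visibility and applies no damage.
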(event `self.ReceiveBeginPlay`
  ;[1 1 1] Create Player Reference
  (bind _asbp_third_person_character (cast `/Game/ThirdPerson/Blueprints/BP_ThirdPersonCharacter` (`GameplayStatics.GetPlayerCharacter` 0)))
  (set `self.PlayerReference` _asbp_third_person_character))

(event `self.BC_FireOutlet.OnComponentBeginOverlap`
  (params (OverlappedComponent :type "PrimitiveComponent Object Reference") (OtherActor :type "Actor Object Reference") (OtherComp :type "PrimitiveComponent Object Reference") (OtherBodyIndex :type Integer) (bFromSweep :type Boolean) (SweepResult :type "HitResult Structure (by ref)"))
  ;[1 1 1] Turn Fire ON (Visibility to On)
  (if (== OtherActor (`self.PlayerReference`))
    (`KismetSystemLibrary.Delay` 0.2)
    (`SceneComponent.SetVisibility` (`self.FireOut`) true false)))

(event `self.BC_FireOutlet.OnComponentEndOverlap`
  (params (OverlappedComponent :type "PrimitiveComponent Object Reference") (OtherActor :type "Actor Object Reference") (OtherComp :type "PrimitiveComponent Object Reference") (OtherBodyIndex :type Integer))
  ;[1 1 1] Turn Fire OFF (Visibility to Off)
  (if (== OtherActor (`self.PlayerReference`))
    (`KismetSystemLibrary.Delay` 1.0)
    (`SceneComponent.SetVisibility` (`self.FireOut`) false false)))

(fn `UserConstructionScript`)